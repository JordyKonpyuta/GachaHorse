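; BP_Checkpoint is a horse racing checkpoint that enforces passing order when a BP_HorseCharacter overlaps it.
; A correctly ordered hit saves the Arrow transform as the respawn point and either advances the horse's index or, at the end line, finishes the race.
; The last checkpoint hides the race UI.
; Out-of-order hits on last or end checkpoints ragdoll horses with zero index and negative MainTimer, then reset target speed.
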(event `self.ReceiveActorBeginOverlap`
  (params (OtherActor :type "Actor Object Reference"))
  (bind _asbp_horse_character (cast `/Game/HorseRacing/BP_HorseCharacter` OtherActor))
  (bind _checkpointindex (`/Game/HorseRacing/BP_HorseCharacter.CheckPointIndex` _asbp_horse_character))
  (if (== _checkpointindex (- (`self.Index`) 1))
    (if (`self.IsEndLine`)
      (set `/Game/HorseRacing/BP_HorseCharacter.CheckPointIndex` 0 _asbp_horse_character)
      (`KismetSystemLibrary.K2_ClearAndInvalidateTimerHandle` (`/Game/HorseRacing/BP_HorseCharacter.TimerHandle` _asbp_horse_character))
      (`/Game/HorseRacing/BP_HorseCharacter.FinishRace` _asbp_horse_character)
      (else
        (set `/Game/HorseRacing/BP_HorseCharacter.CheckPointIndex` (`self.Index`) _asbp_horse_character)
        (if (`self.IsLast`)
          (`/Game/HorseRacing/WBP_Race.HideUI` (`/Game/HorseRacing/BP_HorseCharacter.RaceUI_Ref` _asbp_horse_character)))))
    (set `/Game/HorseRacing/BP_HorseCharacter.LastRespawnPoint` (`SceneComponent.K2_GetComponentToWorld` (`self.Arrow`)) _asbp_horse_character)
    (elif (and (== _checkpointindex 0) (< (`/Game/HorseRacing/BP_HorseCharacter.MainTimer` _asbp_horse_character) 0.0))
      (if (or (`self.IsEndLine`) (`self.IsLast`))
        (`/Game/HorseRacing/BP_HorseCharacter.Ragdoll` _asbp_horse_character)
        (set `/Game/HorseRacing/BP_HorseCharacter.TargetSpeedIndex` 1 _asbp_horse_character)
        (`/Game/HorseRacing/BP_HorseCharacter.SetTargetSpeed` _asbp_horse_character)))))

(fn `UserConstructionScript`)