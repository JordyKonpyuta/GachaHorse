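; Player horse-and-rider character for a racing game, with gamepad steering, stepped target speeds on a shift cooldown, and charged jumps.
; Tick drives movement input toward the target speed, adjusted by traced slope direction, and damps sideways drift.
; Hit normals decide collisions: frontal ones stop or ragdoll and respawn the horse, side ones deflect it.
; BeginPlay applies stat levels and creates the race HUD; FinishRace shows results and swings the camera.
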(event `FinishRace`
  (bind _springarm (`self.SpringArm`))
  (set `self.TargetSpeedIndex` 1)
  (`self.SetTargetSpeed`)
  (bind _returnvalue (`|CreateWidget` "/Game/HorseRacing/WBP_Finish.WBP_Finish_C"))
  (bind _output_get (set `self.FinishUI_Ref` _returnvalue))
  (`UserWidget.AddToViewport` _output_get 0)
  (set `/Game/HorseRacing/WBP_Finish.Parent` self _output_get)
  (`/Game/HorseRacing/WBP_Finish.Start` _output_get)
  (bind (_direction _newtrack_0) (`Timeline|Timeline` :!via `PlayFromStart`)
    (:`Update`
      (set `SpringArmComponent.TargetArmLength` (+ (* _newtrack_0 -200.0) 600.0) _springarm)
      (`SceneComponent.K2_SetRelativeRotation` _springarm (`KismetMathLibrary.MakeRotator` 0.0 -20.0 (* _newtrack_0 -135.0)) false false))))

(event `self.ReceiveHit`
  (params (MyComp :type "PrimitiveComponent Object Reference") (Other :type "Actor Object Reference") (OtherComp :type "PrimitiveComponent Object Reference") (bSelfMoved :type Boolean) (HitLocation :type "Vector Structure") (HitNormal :type "Vector Structure") (NormalImpulse :type "Vector Structure") (Hit :type "HitResult Structure (by ref)"))
  (bind _charactermovement (`self.CharacterMovement`))
  (bind _returnvalue (`KismetMathLibrary.MakeVector2D` (.x HitNormal) (.y HitNormal)))
  (bind _returnvalue_2 (`KismetMathLibrary.DotProduct2D` _returnvalue (`KismetMathLibrary.MakeVector2D` (.x (`self.GetActorForwardVector`)) (.y (`self.GetActorForwardVector`)))))
  (bind _returnvalue_3 (> (`KismetMathLibrary.DotProduct2D` _returnvalue (`KismetMathLibrary.MakeVector2D` (.x (`self.GetActorRightVector`)) (.y (`self.GetActorRightVector`)))) 0.0))
  (bind _returnvalue_4 (`KismetMathLibrary.SelectFloat` 0.5 -0.5 _returnvalue_3))
  ;[1 1 1] If the Vector2D is small, then the surface is treating as something you can land on
  (if (not (< (`KismetMathLibrary.VSize2D` _returnvalue) 0.35))
    ;[1 1 1] x<-0.5: Frontal -> ragdoll if fast
    (if (< _returnvalue_2 -0.5)
      (if (`NavMovementComponent.IsMovingOnGround` (`self.CharacterMovement`))
        (if (> (`self.CurrentSpeed`) 800.0)
          (`self.Ragdoll`)
          (set `self.TargetSpeedIndex` 1)
          (else
            (`MovementComponent.StopMovementImmediately` (`self.CharacterMovement`))
            (set `self.TargetSpeedIndex` (`KismetMathLibrary.Clamp` (`self.TargetSpeedIndex`) 0 1))))
        (else
          (`self.Ragdoll`)
          (set `self.TargetSpeedIndex` 1)))
      (`self.SetTargetSpeed`)
      (else
        ;[1 1 1] -0.5<=x<=0: Coté -> redirect
        (if (<= _returnvalue_2 0.0)
          (if _returnvalue_3
            _
            (else
              _))
          (`self.AddControllerYawInput` _returnvalue_4)
          (set `MovementComponent.Velocity` (`KismetMathLibrary.RotateAngleAxis` (`MovementComponent.Velocity` _charactermovement) _returnvalue_4 (0.0 0.0 1.0)) _charactermovement)
          (if (> (`self.CurrentSpeed`) 1000.0)
            (set `self.TargetSpeedIndex` (`KismetMathLibrary.Clamp` (`self.TargetSpeedIndex`) 0 4))
            (`self.SetTargetSpeed`)
            (set `self.CanShiftSpeed` false)
            (`KismetSystemLibrary.K2_SetTimerDelegate` (delegate `ResetShift`) (`self.ShiftCooldown`)))
          (else
            ;[1 1 1] x>0: Arrière -> rien
            (`KismetSystemLibrary.PrintString` "Back hit")))))))

(event `Ragdoll`
  (bind _rider (`self.rider`))
  (set `self.IsRagdolling` true)
  (`PrimitiveComponent.SetCollisionEnabled` _rider "QueryAndPhysics")
  (`PrimitiveComponent.SetCollisionEnabled` (`self.horse`) "QueryAndPhysics")
  (`SkeletalMeshComponent.SetAllBodiesSimulatePhysics` _rider true)
  (`SkeletalMeshComponent.SetAllBodiesSimulatePhysics` (`self.horse`) true)
  (`KismetSystemLibrary.K2_SetTimerDelegate` (delegate `StopRagdoll`) 1.0)
  (`MovementComponent.StopMovementImmediately` (`self.CharacterMovement`)))

(event `StopRagdoll`
  (bind _horse (`self.horse`))
  (bind (_lastrespawnpoint_location _lastrespawnpoint_rotation) (`KismetMathLibrary.BreakTransform` (`self.LastRespawnPoint`)))
  (bind _rider (`self.rider`))
  (`PrimitiveComponent.SetCollisionEnabled` _rider "QueryOnly")
  (`PrimitiveComponent.SetCollisionEnabled` (`self.horse`) "QueryOnly")
  (`SkeletalMeshComponent.SetAllBodiesSimulatePhysics` _rider false)
  (`SkeletalMeshComponent.SetAllBodiesSimulatePhysics` (`self.horse`) false)
  (`SceneComponent.K2_AttachToComponent` _horse (`self.Mesh`) "None" "KeepRelative" "KeepRelative" "KeepRelative" true)
  (`SceneComponent.K2_SetRelativeLocationAndRotation` _horse (0.0 0.0 5.0) (struct) false false)
  (`SceneComponent.K2_SetRelativeLocationAndRotation` (`self.rider`) (0.0 0.0 5.0) (struct) false false)
  (`self.K2_SetActorLocation` _lastrespawnpoint_location)
  (`Controller.SetControlRotation` (`self.GetController`) _lastrespawnpoint_rotation)
  (set `self.IsRagdolling` false))

(event `Key|Gamepad_LeftStick_Up`
  (params (Key :type "Key Structure"))
  (bind _targetspeedindex (`self.TargetSpeedIndex`))
  (:`Pressed`
    (if (`NavMovementComponent.IsMovingOnGround` (`self.CharacterMovement`))
      (if (> (`self.SlopeType`) -1)
        (if (not (`self.IsRagdolling`))
          (if (`self.CanShiftSpeed`)
            (if (< _targetspeedindex 5)
              (`/Engine/EditorBlueprintResources/StandardMacros.IncrementInt` _targetspeedindex
                (:`  `
                  (set `self.CanShiftSpeed` false :!label _label)
                  (`KismetSystemLibrary.K2_SetTimerDelegate` (delegate `ResetShift`) (`self.ShiftCooldown`))
                  (`self.SetTargetSpeed`))))))))))

(event `Timer`
  (set `self.MainTimer` (+ (`self.MainTimer`) 0.01)))

(event `Key|Gamepad_LeftStick_Down`
  (params (Key :type "Key Structure"))
  (bind _targetspeedindex (`self.TargetSpeedIndex`))
  (:`Pressed`
    (if (`NavMovementComponent.IsMovingOnGround` (`self.CharacterMovement`))
      (if (< (`self.SlopeType`) 1)
        (if (not (`self.IsRagdolling`))
          (if (`NavMovementComponent.IsMovingOnGround` (`self.CharacterMovement`))
            (if (`self.CanShiftSpeed`)
              (if (> _targetspeedindex 0)
                (`/Engine/EditorBlueprintResources/StandardMacros.DecrementInt` _targetspeedindex
                  (:`  `
                    (goto _label)))))))))))

(event `self.ReceiveBeginPlay`
  (bind _returnvalue (`KismetSystemLibrary.K2_SetTimerDelegate` (delegate `Timer`) 0.01 true))
  (set `self.TimerHandle` _returnvalue)
  (set `self.LastRespawnPoint` (`self.GetTransform`))
  ;[1 1 1] Initialize Acceleration=300+20*AccelLevel
  (set `CharacterMovementComponent.MaxAcceleration` (+ (* (`self.AccelLevel`) 20.0) 300.0) (`self.CharacterMovement`))
  ;[1 1 1] InitializeMaxSpeed=1750+25*SpeedLevel
  (`KismetArrayLibrary.Array_Set` (`self.SpeedTable`) 5 (+ (* (`self.SpeedLevel`) 25.0) 1750.0))
  ;[1 1 1] Initialize TurnRateFactor=20-1*HandlingLevel
  (set `self.TurnRateFactor` (+ (* (`self.HandlingLevel`) 0.005) 0.05))
  (`self.SetTargetSpeed`)
  ;[1 1 1] InitializeWidget
  (bind _returnvalue_2 (`|CreateWidget` "/Game/HorseRacing/WBP_Race.WBP_Race_C"))
  (bind _output_get (set `self.RaceUI_Ref` _returnvalue_2))
  (`UserWidget.AddToViewport` _output_get 0)
  (set `/Game/HorseRacing/WBP_Race.MaxSpeed` (`|GetArrayItem` (`self.SpeedTable`) 5) _output_get)
  (set `/Game/HorseRacing/WBP_Race.ParentHorse` self _output_get))

(event `InputAxisKey|Gamepad_LeftX`
  (params (AxisValue :type "Float (single-precision)"))
  (bind _charactermovement (`self.CharacterMovement`))
  (bind _returnvalue (/ (* AxisValue (`self.TurnRateFactor`)) (`KismetMathLibrary.SelectFloat` 3.0 1.0 (`self.Charging`)) (`KismetMathLibrary.SelectFloat` 1.0 100.0 (`NavMovementComponent.IsMovingOnGround` (`self.CharacterMovement`)))))
  ;[1 1 1] Turn
  (if (not (`self.IsRagdolling`))
    (`self.AddControllerYawInput` _returnvalue)
    (set `MovementComponent.Velocity` (`KismetMathLibrary.RotateAngleAxis` (`MovementComponent.Velocity` _charactermovement) _returnvalue (0.0 0.0 1.0)) _charactermovement)))

(event `ResetShift`
  (set `self.CanShiftSpeed` true))

(event `SetTargetSpeed`
  (set `self.TargetSpeed` (`|GetArrayItem` (`self.SpeedTable`) (`self.TargetSpeedIndex`))))

(event `self.ReceiveTick`
  (params (DeltaSeconds :type "Float (single-precision)"))
  (bind (_returnvalue_x _returnvalue_y) (`KismetMathLibrary.BreakVector` (`self.GetActorForwardVector`)))
  (bind (_returnvalue_x_2 _returnvalue_y_2) (`KismetMathLibrary.BreakVector` (`self.GetActorRightVector`)))
  (bind _returnvalue (`self.GetActorForwardVector`))
  (bind _returnvalue_2 (`self.GetActorRightVector`))
  (bind (_velocity_x _velocity_y) (`KismetMathLibrary.BreakVector` (`MovementComponent.Velocity` (`self.CharacterMovement`))))
  (bind _returnvalue_3 (`KismetMathLibrary.MakeVector2D` _velocity_x _velocity_y))
  (`KismetSystemLibrary.PrintString` (`KismetStringLibrary.Conv_BoolToString` (`NavMovementComponent.IsMovingOnGround` (`self.CharacterMovement`))) true true (struct :`G` 0.66 :`B` 1.0 :`A` 1.0) 0.0)
  (`self.SlopeCheck`)
  (`self.ChargeTime` DeltaSeconds)
  (set `self.CurrentSpeed` (`KismetMathLibrary.DotProduct2D` _returnvalue_3 (`KismetMathLibrary.MakeVector2D` _returnvalue_x _returnvalue_y)))
  (set `self.SideSpeed` (`KismetMathLibrary.DotProduct2D` _returnvalue_3 (`KismetMathLibrary.MakeVector2D` _returnvalue_x_2 _returnvalue_y_2)))
  (if (and (not (`self.IsRagdolling`)) (`NavMovementComponent.IsMovingOnGround` (`self.CharacterMovement`)))
    ;[1 1 1] ForwardSpeed
    (if (< (`self.CurrentSpeed`) (* (`self.TargetSpeed`) (+ 1.0 (* (`self.SlopeType`) 0.15))))
      (`self.AddMovementInput` _returnvalue (+ (* (`self.SlopeType`) 0.5) 1.0))
      (else
        (`self.AddMovementInput` _returnvalue (+ (* (`self.SlopeType`) 0.5) -1.0))))
    ;[1 1 1] LateralVelocityNerf
    (if (not (`KismetMathLibrary.NearlyEqual_FloatFloat` (`self.SideSpeed`) 0.0 0.1))
      (if (< (`self.SideSpeed`) 0.0)
        (`self.AddMovementInput` _returnvalue_2 2.0)
        (else
          (`self.AddMovementInput` _returnvalue_2 -2.0))))))

(event `SlopeCheck`
  (bind _returnvalue (`self.K2_GetActorLocation`))
  ;[1 1 1] SlopeCheck
  (if (`NavMovementComponent.IsMovingOnGround` (`self.CharacterMovement`))
    (bind _outhit (`KismetSystemLibrary.LineTraceSingle` _returnvalue (- _returnvalue (0.0 0.0 1000.0)) "TraceTypeQuery1"))
    (bind _returnvalue_2 (`KismetMathLibrary.Dot_VectorVector` (`.Normal` (`GameplayStatics.BreakHitResult` _outhit)) (`self.GetActorForwardVector`)))
    (if (`KismetMathLibrary.NearlyEqual_FloatFloat` _returnvalue_2)
      (set `self.SlopeType` 0)
      (elif (> _returnvalue_2 0.0)
        (set `self.SlopeType` 1)
        (else
          (set `self.SlopeType` -1))))
    (else
      (set `self.SlopeType` 0))))

(event `ChargeTime`
  (params (Delta :type "Float (double-precision)"))
  ;[1 1 1] Charging
  (if (`self.Charging`)
    (bind _output_get (set `self.ChargeTimer` (`KismetMathLibrary.FClamp` (+ (`self.ChargeTimer`) Delta) 0.0 (`self.MaxChargeTime`))))
    (set `CharacterMovementComponent.JumpZVelocity` (* (/ _output_get (`self.MaxChargeTime`)) 450.0) (`self.CharacterMovement`))))

(event `self.OnLanded`
  (params (Hit :type "HitResult Structure (by ref)"))
  ;[1 1 1] On landed
  (bind (_direction _newtrack_0) (`Timeline|CapsuleSizeTimeline` :!via `PlayFromStart`)
    (:`Update`
      (`CapsuleComponent.SetCapsuleSize` (`self.CapsuleComponent`) 34.0 (+ (* _newtrack_0 46.0) 34.0) true))))

(event `Key|Gamepad_FaceButton_Bottom`
  (params (Key :type "Key Structure"))
  (bind _returnvalue (not (`self.IsRagdolling`)))
  (bind _returnvalue_2 (`NavMovementComponent.IsMovingOnGround` (`self.CharacterMovement`)))
  ;[1 1 1] Jumping
  (:`Pressed`
    (if _returnvalue
      (if (and (not (`self.Charging`)) _returnvalue_2)
        (set `self.Charging` true)
        (set `self.ChargeTimer` 0.0)
        (`/Game/HorseRacing/WBP_Race.ShowCharge` (`self.RaceUI_Ref`)))))
  (:`Released`
    (if _returnvalue_2
      (if (and (> (`CharacterMovementComponent.JumpZVelocity` (`self.CharacterMovement`)) 325.0) (> (`self.CurrentSpeed`) 750.0) _returnvalue)
        (`self.Jump`)
        (`CapsuleComponent.SetCapsuleSize` (`self.CapsuleComponent`) 34.0 34.0 true))
      (set `self.Charging` false)
      (`/Game/HorseRacing/WBP_Race.HideCharge` (`self.RaceUI_Ref`)))))

(fn `UserConstructionScript`)