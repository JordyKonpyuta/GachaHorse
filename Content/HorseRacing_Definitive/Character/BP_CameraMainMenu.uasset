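; BP_CameraMainMenu is the main menu camera that glides between menu positions in the horse racing game.
; On BeginPlay it registers with BP_MainMenuController, becomes the player's view target and snaps to the PositionMenu transform.
; CameraMovement stores a destination and widget class, then starts a looping timer that eases the camera there with TInterpTo.
; When nearly arrived, it clears the timer and adds the requested widget to the viewport.
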(event `self.ReceiveBeginPlay`
  (bind _returnvalue (`GameplayStatics.GetPlayerController` 0))
  (bind _asbp_main_menu_controller (cast `/Game/HorseRacing_Definitive/Character/BP_MainMenuController` _returnvalue))
  (set `/Game/HorseRacing_Definitive/Character/BP_MainMenuController.CameraRef` self _asbp_main_menu_controller)
  (`PlayerController.SetViewTargetWithBlend` _returnvalue self 0.0 "VTBlend_Linear" 0.0 false)
  (`self.K2_SetActorTransform` (`self.GetTransform` (`self.PositionMenu`))))

(event `CameraMovement`
  (params (Destination :type "Transform Structure") (WidgetToCreate :type "UserWidget Class Reference"))
  (set `self.Destination` Destination)
  (set `self.WidgetToCreate` WidgetToCreate)
  (bind _returnvalue (`KismetSystemLibrary.K2_SetTimerDelegate` (delegate `MoveCamera`) 0.01 true))
  (set `self.PositionTimerHandler` _returnvalue))

(event `MoveCamera`
  (bind _returnvalue (`self.GetTransform`))
  (`self.K2_SetActorTransform` (`KismetMathLibrary.TInterpTo` _returnvalue (`self.Destination`) (`GameplayStatics.GetWorldDeltaSeconds`) 5.0))
  (if (`KismetMathLibrary.NearlyEqual_TransformTransform` _returnvalue (`self.Destination`) 5.0 5.0)
    (`KismetSystemLibrary.K2_ClearAndInvalidateTimerHandle` (`self.PositionTimerHandler`))
    (bind _returnvalue_2 (`|CreateWidget` (`self.WidgetToCreate`)))
    (`UserWidget.AddToViewport` _returnvalue_2 0)))

(fn `UserConstructionScript`)