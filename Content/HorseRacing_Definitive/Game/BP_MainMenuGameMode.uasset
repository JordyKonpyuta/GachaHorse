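; Main menu game mode for the horse racing game that fills the summoning, rankings and management screens.
; Summon events create the summoning widget and look up pulled horses or equipment by ID in data tables to fill card slots.
; Ranking events add rows with formatted race times to track selection.
; Selection events show stats, level and rarity, with shard or scrap upgrade costs from nested Selects by level and rarity.
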(event `DisplaySummonScreen`
  (params (IsSummon10 :type Boolean))
  (bind _returnvalue (`|CreateWidget` "/Game/HorseRacing_Definitive/Widgets/WBP_SummoningScreen.WBP_SummoningScreen_C"))
  (bind _output_get (set `self.SummoningScreenRef` _returnvalue))
  (set `/Game/HorseRacing_Definitive/Widgets/WBP_SummoningScreen.IsSummon10` IsSummon10 _output_get)
  (`UserWidget.AddToViewport` _output_get 0))

(event `self.DisplaySummonResults`
  (params (bIsHorses :type Boolean) (ThingID :type Integer))
  (bind _outrownames (`DataTableFunctionLibrary.GetDataTableRowNames` (select `bool` bIsHorses :`false` "/Game/HorseRacing_Definitive/DataTables/AllEquipmentData.AllEquipmentData" :`true` "/Game/HorseRacing_Definitive/DataTables/AllHorsesData.AllHorsesData" :!type "DataTable Object Reference")))
  (for _array_element _outrownames :!label _label
    (if bIsHorses
      (bind _returnvalue (`|GetDataTableRow` "/Game/HorseRacing_Definitive/DataTables/AllHorsesData.AllHorsesData" _array_element)
        (:`then`
          (bind (_bhorsepossessed _shardnumber _level _horseid _rarity _horsename _horsepicture) (break `HorseDataStruct` _returnvalue))
          (if (== ThingID _horseid)
            (`/Game/HorseRacing_Definitive/Widgets/WBP_SummoningScreen.InitCardSlots` (`self.SummoningScreenRef`) _bhorsepossessed _horsename _rarity (`|ConvertAsset` _horsepicture) _level bIsHorses)
            (`self.Break`))))
      (else
        (bind _returnvalue_2 (`|GetDataTableRow` "/Game/HorseRacing_Definitive/DataTables/AllEquipmentData.AllEquipmentData" _array_element)
          (:`then`
            (bind (_bequipmentpossessed _level_2 _equipmentid _rarity_2 _equipmentname _equipmentpicture) (break `EquipDataStruct` _returnvalue_2))
            (if (== _equipmentid ThingID)
              (`/Game/HorseRacing_Definitive/Widgets/WBP_SummoningScreen.InitCardSlots` (`self.SummoningScreenRef`) _bequipmentpossessed _equipmentname _rarity_2 (`|ConvertAsset` _equipmentpicture) _level_2 bIsHorses)
              (`self.Break`))))))))

(event `Break`
  (goto _label :!via `Break`))

(event `self.DisplayRankingsResults`
  (params (bIsPlayer :type Boolean) (CurRankName :type Name) (CurRankTime :type "Float (single-precision)"))
  (bind _returnvalue (`|CreateWidget` "/Game/HorseRacing_Definitive/Widgets/WBP_Rank.WBP_Rank_C"))
  (`PanelWidget.AddChild` (`/Game/HorseRacing_Definitive/Widgets/WBP_TrackSelection.ScrollBox_Rankings` (`self.TrackSelectionRef`)) _returnvalue)
  (`Widget.SetVisibility` (`/Game/HorseRacing_Definitive/Widgets/WBP_Rank.Image_PlayerIcon` _returnvalue) (select `bool` bIsPlayer :`false` "Hidden" :`true` "SelfHitTestInvisible" :!type "ESlateVisibility Enum"))
  (`TextBlock.SetText` (`/Game/HorseRacing_Definitive/Widgets/WBP_Rank.Text_Name` _returnvalue) (`KismetTextLibrary.Conv_NameToText` CurRankName))
  (`TextBlock.SetText` (`/Game/HorseRacing_Definitive/Widgets/WBP_Rank.Text_Time` _returnvalue) (`|FormatText` "{m} : {s} : {ms}" (`KismetTextLibrary.Conv_IntToText` (`KismetMathLibrary.FFloor` (/ CurRankTime 60.0)) false true 2 2) (`KismetTextLibrary.Conv_IntToText` (`KismetMathLibrary.FFloor` (mod CurRankTime 60.0)) false true 2 2) (`KismetTextLibrary.Conv_IntToText` (`KismetMathLibrary.FFloor` (* (- CurRankTime (`KismetMathLibrary.FFloor` 0.0)) 1000.0)) false true 3 3))))

(event `self.SelectHorseWidget`
  (params (HorseDisplayed :type "HorseDataStruct Structure"))
  (bind (_bhorsepossessed _shardnumber _level _horseid _rarity _horsename _horsepicture _accelerationperlevel _speedperlevel _handlingperlevel) (break `HorseDataStruct` HorseDisplayed))
  (bind _managementscreenref (`self.ManagementScreenRef`))
  (bind _returnvalue (- _level 1))
  (`ProgressBar.SetPercent` (`/Game/HorseRacing_Definitive/Widgets/WBP_HorseManagement.PB_Speed` (`self.ManagementScreenRef`)) (/ (`|GetArrayItem` _speedperlevel _returnvalue) (`self.Stat Percentage Divider`)))
  (`ProgressBar.SetPercent` (`/Game/HorseRacing_Definitive/Widgets/WBP_HorseManagement.PB_Accel` (`self.ManagementScreenRef`)) (/ (`|GetArrayItem` _accelerationperlevel _returnvalue) (`self.Stat Percentage Divider`)))
  (`ProgressBar.SetPercent` (`/Game/HorseRacing_Definitive/Widgets/WBP_HorseManagement.PB_Handling` (`self.ManagementScreenRef`)) (/ (`|GetArrayItem` _handlingperlevel _returnvalue) (`self.Stat Percentage Divider`)))
  (`ProgressBar.SetPercent` (`/Game/HorseRacing_Definitive/Widgets/WBP_HorseManagement.PB_Level` (`self.ManagementScreenRef`)) (/ _shardnumber (select `int` _level :`0` 1.0 :`1` 1.0 :`2` 2.0 :`3` 4.0 :`4` 8.0 :`5` 16.0 :`6` 1.0)))
  (`TextBlock.SetText` (`/Game/HorseRacing_Definitive/Widgets/WBP_HorseManagement.Text_HorseLevel` _managementscreenref) (`|FormatText` "Level : {x}" (`KismetMathLibrary.SelectText` (`KismetTextLibrary.Conv_IntToText` _level) "MAX" (< _level 6))))
  (`TextBlock.SetText` (`/Game/HorseRacing_Definitive/Widgets/WBP_HorseManagement.Text_HorseName` _managementscreenref) (`KismetTextLibrary.Conv_StringToText` _horsename))
  (`TextBlock.SetText` (`/Game/HorseRacing_Definitive/Widgets/WBP_HorseManagement.Text_HorseRarity` _managementscreenref) (select `int` _rarity :`0` "Common" :`1` "Uncommon" :`2` "Rare" :!type "Text"))
  (`TextBlock.SetText` (`/Game/HorseRacing_Definitive/Widgets/WBP_HorseManagement.Text_Shards` _managementscreenref) (`|FormatText` "{shards} / {Necessary Shards}" _shardnumber (select `int` _level :`0` 1.0 :`1` 1.0 :`2` 2.0 :`3` 4.0 :`4` 8.0 :`5` 16.0 :`6` 1.0))))

(event `self.SelectEquipWidget`
  (params (EquipDisplayed :type "EquipDataStruct Structure"))
  (bind (_bequipmentpossessed _level _equipmentid _rarity _equipmentname _equipmentpicture _accelerationperlevel _speedperlevel _handlingperlevel) (break `EquipDataStruct` EquipDisplayed))
  (bind _managementscreenref (`self.ManagementScreenRef`))
  (bind _managementscreenref_2 (`self.ManagementScreenRef`))
  (bind _managementscreenref_3 (`self.ManagementScreenRef`))
  (bind _returnvalue (- _level 1))
  (bind _text_levelmax (`/Game/HorseRacing_Definitive/Widgets/WBP_HorseManagement.Text_LevelMax` _managementscreenref_2))
  (bind _hp_equipmentmode (`/Game/HorseRacing_Definitive/Widgets/WBP_HorseManagement.HP_EquipmentMode` _managementscreenref_2))
  (`ProgressBar.SetPercent` (`/Game/HorseRacing_Definitive/Widgets/WBP_HorseManagement.PB_Speed` (`self.ManagementScreenRef`)) (/ (`|GetArrayItem` _speedperlevel _returnvalue) (`self.Stat Percentage Divider`)))
  (`ProgressBar.SetPercent` (`/Game/HorseRacing_Definitive/Widgets/WBP_HorseManagement.PB_Accel` (`self.ManagementScreenRef`)) (/ (`|GetArrayItem` _accelerationperlevel _returnvalue) (`self.Stat Percentage Divider`)))
  (`ProgressBar.SetPercent` (`/Game/HorseRacing_Definitive/Widgets/WBP_HorseManagement.PB_Handling` (`self.ManagementScreenRef`)) (/ (`|GetArrayItem` _handlingperlevel _returnvalue) (`self.Stat Percentage Divider`)))
  (`TextBlock.SetText` (`/Game/HorseRacing_Definitive/Widgets/WBP_HorseManagement.Text_HorseLevel` _managementscreenref) (`|FormatText` "Level : {x}" (`KismetMathLibrary.SelectText` (`KismetTextLibrary.Conv_IntToText` _level) "MAX" (< _level 6))))
  (`TextBlock.SetText` (`/Game/HorseRacing_Definitive/Widgets/WBP_HorseManagement.Text_HorseName` _managementscreenref) (`KismetTextLibrary.Conv_StringToText` _equipmentname))
  (`TextBlock.SetText` (`/Game/HorseRacing_Definitive/Widgets/WBP_HorseManagement.Text_HorseRarity` _managementscreenref) (select `int` _rarity :`0` "Common" :`1` "Uncommon" :`2` "Rare" :!type "Text"))
  (`TextBlock.SetText` (`/Game/HorseRacing_Definitive/Widgets/WBP_HorseManagement.Text_Scraps_Owned` _managementscreenref_3) (`KismetTextLibrary.Conv_IntToText` (`BaseGameInstance.GetScrap` (`self.InstanceRef`))))
  (`TextBlock.SetText` (`/Game/HorseRacing_Definitive/Widgets/WBP_HorseManagement.Text_Scraps_Needed` _managementscreenref_3) (`KismetTextLibrary.Conv_IntToText` (select `int` _level :`0` 1 :`1` (select `int` _rarity :`0` 2 :`1` 5 :`2` 25) :`2` (select `int` _rarity :`0` 4 :`1` 10 :`2` 50) :`3` (select `int` _rarity :`0` 8 :`1` 20 :`2` 100) :`4` (select `int` _rarity :`0` 16 :`1` 40 :`2` 200) :`5` (select `int` _rarity :`0` 32 :`1` 80 :`2` 400) :`6` (select `int` _rarity :`0` 1 :`1` 1 :`2` 1))))
  (if (>= _level 6)
    (`Widget.SetVisibility` _text_levelmax "SelfHitTestInvisible")
    (`Widget.SetVisibility` _hp_equipmentmode "Hidden")
    (else
      (`Widget.SetVisibility` _text_levelmax "Hidden")
      (`Widget.SetVisibility` _hp_equipmentmode "SelfHitTestInvisible"))))

(fn `UserConstructionScript`)