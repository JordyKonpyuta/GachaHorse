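; BP_HorseRunGamemode is the horse racing game mode that owns and drives the UI, creating the main menu widget on Map_MainMenu and the race HUD on other levels.
; Its events forward countdown and timer updates to the stored HUD reference.
; Victory switches the HUD to a results panel with time, rank and reward, highlighting new records when rank increases.
; Three mission events play clear animations and animate prize money being added.
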(event `self.WidgetTimerUpdate`
  (params (CurrentTimer :type "Float (single-precision)"))
  (`/Game/HorseRacing_Definitive/Widgets/WBP_HUD.SetTimerText` (`self.HUD_Ref`) CurrentTimer))

(event `self.WidgetVictory`
  (params (CurrentTimer :type "Float (single-precision)") (OldRank :type Integer) (NewRank :type Integer) (RewardAmount :type Integer))
  (bind _returnvalue (> NewRank OldRank))
  (bind _hud_ref (`self.HUD_Ref`))
  (bind _hud_ref_2 (`self.HUD_Ref`))
  (`WidgetSwitcher.SetActiveWidgetIndex` (`/Game/HorseRacing_Definitive/Widgets/WBP_HUD.WidgetSwitcher_HUD` _hud_ref_2) 1)
  (`/Game/HorseRacing_Definitive/Widgets/WBP_HUD.SetVictoryTimer` _hud_ref_2 CurrentTimer)
  (`KismetSystemLibrary.PrintString` (`KismetStringLibrary.Concat_StrStr` "Old Rank : " (`KismetStringLibrary.Conv_IntToString` OldRank) " ; New Rank : " (`KismetStringLibrary.Conv_IntToString` NewRank) " ; Reward Ammount : " (`KismetStringLibrary.Conv_IntToString` RewardAmount)) true true (struct :`G` 0.66 :`B` 1.0 :`A` 1.0) 1000.0)
  (`Widget.SetVisibility` (`/Game/HorseRacing_Definitive/Widgets/WBP_HUD.Text_NewRecord` (`self.HUD_Ref`)) (select `bool` _returnvalue :`false` "Hidden" :`true` "SelfHitTestInvisible" :!type "ESlateVisibility Enum"))
  (`Widget.SetVisibility` (`/Game/HorseRacing_Definitive/Widgets/WBP_HUD.Text_NewRank` (`self.HUD_Ref`)) (select `bool` _returnvalue :`false` "Hidden" :`true` "SelfHitTestInvisible" :!type "ESlateVisibility Enum"))
  (`Widget.SetVisibility` (`/Game/HorseRacing_Definitive/Widgets/WBP_HUD.Image_NewRank` (`self.HUD_Ref`)) (select `bool` _returnvalue :`false` "Hidden" :`true` "SelfHitTestInvisible" :!type "ESlateVisibility Enum"))
  (`TextBlock.SetText` (`/Game/HorseRacing_Definitive/Widgets/WBP_HUD.Text_NewRank` (`self.HUD_Ref`)) (`|FormatText` "New rank : {x}" NewRank))
  (`TextBlock.SetText` (`/Game/HorseRacing_Definitive/Widgets/WBP_HUD.Text_ActualRank` (`self.HUD_Ref`)) (select `bool` _returnvalue :`false` (`|FormatText` "Actual rank : {x}" OldRank) :`true` (`|FormatText` "Old rank : {x}" OldRank)))
  (`TextBlock.SetText` (`/Game/HorseRacing_Definitive/Widgets/WBP_HUD.Text_Reward` (`self.HUD_Ref`)) (`|FormatText` "Rewards : {x}" RewardAmount))
  (`UserWidget.PlayAnimation` _hud_ref (select `bool` _returnvalue :`false` (`/Game/HorseRacing_Definitive/Widgets/WBP_HUD.PopUpFinish` _hud_ref) :`true` (`/Game/HorseRacing_Definitive/Widgets/WBP_HUD.PopUpFinish_NewRecord` _hud_ref)) 0.0 1 "Forward" 1.0 false))

(event `self.Widget_ReadyToGo`
  (params (TimeBeforeGo :type Integer))
  (`/Game/HorseRacing_Definitive/Widgets/WBP_HUD.StartCount` (`self.HUD_Ref`) TimeBeforeGo))

(event `self.SetupWidgets`
  (bind _returnvalue (`GameplayStatics.GetCurrentLevelName` true))
  (if (`KismetStringLibrary.NotEqual_StrStr` _returnvalue "Map_MainMenu")
    (bind _returnvalue_2 (`|CreateWidget` "/Game/HorseRacing_Definitive/Widgets/WBP_HUD.WBP_HUD_C"))
    (bind _output_get (set `self.HUD_Ref` _returnvalue_2))
    (`UserWidget.AddToViewport` _output_get 0)
    (else
      (bind _returnvalue_3 (`|CreateWidget` "/Game/HorseRacing_Definitive/Widgets/WBP_Menu.WBP_Menu_C"))
      (`UserWidget.AddToViewport` _returnvalue_3 0))))

(event `self.FirstMissionWidget`
  (params (bAnimation :type Boolean) (Prize :type Integer))
  (bind _hud_ref (`self.HUD_Ref`))
  (if bAnimation
    (`UserWidget.PlayAnimation` _hud_ref (`/Game/HorseRacing_Definitive/Widgets/WBP_HUD.MissionClear_1` _hud_ref) 0.0 1 "Forward" 1.0 false)
    (`/Game/HorseRacing_Definitive/Widgets/WBP_HUD.SmoothMoneyAdding` (`self.HUD_Ref`) Prize)))

(event `self.SecondMissionWidget`
  (params (bAnimation :type Boolean) (Prize :type Integer))
  (bind _hud_ref (`self.HUD_Ref`))
  (if bAnimation
    (`UserWidget.PlayAnimation` _hud_ref (`/Game/HorseRacing_Definitive/Widgets/WBP_HUD.MissionClear_2` _hud_ref) 0.0 1 "Forward" 1.0 false)
    (`/Game/HorseRacing_Definitive/Widgets/WBP_HUD.SmoothMoneyAdding` (`self.HUD_Ref`) Prize)))

(event `self.ThirdMissionWidget`
  (params (bAnimation :type Boolean) (Prize :type Integer))
  (bind _hud_ref (`self.HUD_Ref`))
  (if bAnimation
    (`UserWidget.PlayAnimation` _hud_ref (`/Game/HorseRacing_Definitive/Widgets/WBP_HUD.MissionClear_3` _hud_ref) 0.0 1 "Forward" 1.0 false)
    (`/Game/HorseRacing_Definitive/Widgets/WBP_HUD.SmoothMoneyAdding` (`self.HUD_Ref`) Prize)))

(fn `UserConstructionScript`)