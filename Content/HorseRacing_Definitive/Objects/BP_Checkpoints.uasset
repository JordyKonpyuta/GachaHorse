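; BP_Checkpoints is a horse racing checkpoint that sets its visual effect according to its checkpoint type.
; On BeginPlay, the type selects a spline Niagara system for generic, last or start checkpoints.
; A start checkpoint then runs a timed sequence, hiding its lightning effect briefly before reappearing with the holy effect used by the last checkpoint.
; The graph contains only this visual logic, with no overlap or race-progress handling.
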(event `self.ReceiveBeginPlay`
  (bind _currentcheckpointtype (`self.CurrentCheckpointType`))
  (bind _niagara (`self.Niagara`))
  (`NiagaraComponent.SetAsset` (`self.Niagara`) (select `ECheckpointType` _currentcheckpointtype :`Generic` "/Game/HorseRacing_Definitive/VFX/_SplineVFX/NS/NS_Spline_Wind.NS_Spline_Wind" :`LastGen` "/Game/HorseRacing_Definitive/VFX/_SplineVFX/NS/NS_Spline_Holy.NS_Spline_Holy" :`Start` "/Game/HorseRacing_Definitive/VFX/_SplineVFX/NS/NS_Spline_ElectricLightning.NS_Spline_ElectricLightning" :!type "NiagaraSystem Object Reference") true)
  (if (`|EnumEquality` _currentcheckpointtype "Start")
    (`KismetSystemLibrary.Delay` 7.0)
    (`SceneComponent.SetVisibility` (`self.Niagara`) false false)
    (`KismetSystemLibrary.Delay` 2.0)
    (`SceneComponent.SetVisibility` _niagara true false)
    (`NiagaraComponent.SetAsset` _niagara "/Game/HorseRacing_Definitive/VFX/_SplineVFX/NS/NS_Spline_Holy.NS_Spline_Holy" true)))

(fn `UserConstructionScript`)