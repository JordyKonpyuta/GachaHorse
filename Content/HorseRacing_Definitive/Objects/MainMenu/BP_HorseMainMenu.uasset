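; BP_HorseMainMenu is a display horse for the main menu that shows either the chosen or the viewed horse and its equipment.
; On BeginPlay it loops one animation on the body, hair, reins, saddle and belt meshes, and registers itself in BP_MainMenuController's Horses list.
; UpdateHorseVisual applies materials from the GameInstance's horse and equipment data, picking Viewed or Chosen data via IsManagementScreen.
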(event `self.ReceiveBeginPlay`
  (`SkeletalMeshComponent.PlayAnimation` (`self.Horse_Base`) (`self.AnimationToPlay`) true)
  (`SkeletalMeshComponent.PlayAnimation` (`self.Horse_Hair`) (`self.AnimationToPlay`) true)
  (`SkeletalMeshComponent.PlayAnimation` (`self.Horse_Reins`) (`self.AnimationToPlay`) true)
  (`SkeletalMeshComponent.PlayAnimation` (`self.Horse_Saddle`) (`self.AnimationToPlay`) true)
  (`SkeletalMeshComponent.PlayAnimation` (`self.Horse_Belts`) (`self.AnimationToPlay`) true)
  (`KismetArrayLibrary.Array_AddUnique` (`/Game/HorseRacing_Definitive/Character/BP_MainMenuController.Horses` (cast `/Game/HorseRacing_Definitive/Character/BP_MainMenuController` (`GameplayStatics.GetPlayerController` 0) :!pure true)) self)
  (`self.UpdateHorseVisual`))

(event `UpdateHorseVisual`
  (bind _asbp_game_instance (cast `/Game/HorseRacing_Definitive/Game/BP_GameInstance` (`GameplayStatics.GetGameInstance`) :!pure true))
  (bind ((`HorseMaterial` _horsematerial) (`HairMaterial` _hairmaterial)) (break `HorseDataStruct` (select `bool` (`self.IsManagementScreen`) :`false` (`BaseGameInstance.ChosenHorseData` _asbp_game_instance) :`true` (`BaseGameInstance.ViewedHorseData` _asbp_game_instance))))
  (bind _output (`|ConvertAsset` _hairmaterial))
  (`PrimitiveComponent.SetMaterial` (`self.Horse_Base`) 0 (`|ConvertAsset` _horsematerial))
  (`PrimitiveComponent.SetMaterial` (`self.Horse_Hair`) 0 _output)
  (`PrimitiveComponent.SetMaterial` (`self.Horse_Reins`) 0 (`|ConvertAsset` (`.EquipMaterial` (break `EquipDataStruct` (select `bool` (`self.IsManagementScreen`) :`false` (`BaseGameInstance.ChosenEquipData` _asbp_game_instance) :`true` (`BaseGameInstance.ViewedEquipData` _asbp_game_instance))))))
  (`PrimitiveComponent.SetMaterial` (`self.Horse_Saddle`) 0 (`|ConvertAsset` (`.EquipMaterial` (break `EquipDataStruct` (select `bool` (`self.IsManagementScreen`) :`false` (`BaseGameInstance.ChosenEquipData` _asbp_game_instance) :`true` (`BaseGameInstance.ViewedEquipData` _asbp_game_instance))))))
  (`PrimitiveComponent.SetMaterial` (`self.Horse_Belts`) 0 (`|ConvertAsset` (`.EquipMaterial` (break `EquipDataStruct` (select `bool` (`self.IsManagementScreen`) :`false` (`BaseGameInstance.ChosenEquipData` _asbp_game_instance) :`true` (`BaseGameInstance.ViewedEquipData` _asbp_game_instance))))))
  (`KismetSystemLibrary.PrintString` (`KismetSystemLibrary.GetDisplayName` _output)))

(fn `UserConstructionScript`)